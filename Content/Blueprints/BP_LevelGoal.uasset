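; BP_LevelGoal is a level goal trigger that ends the level when the player reaches it.
; A box overlap checks for the player character, then shows the end-of-level screen through the UI.
; It also turns off the character's play mode, shows the mouse cursor with Game and UI input, and calls the timer widget's StartTimer with false.
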(event OnComponentBeginOverlap(Box2)
  (params (OverlappedComponent :type Primitive%20Component%20Object%20Reference) (OtherActor :type Actor%20Object%20Reference) (OtherComp :type Primitive%20Component%20Object%20Reference) (OtherBodyIndex :type Integer) (bFromSweep :type Boolean) (SweepResult :type Hit%20Result%20Structure%20%28by%20ref%29))
  (if (== OtherActor (Game|GetPlayerCharacter 0))
    (Default|ShowHUB (CallFunction|GetUI) (Variables|Default|GetEndOfLevel))
    (Default|SetPlayMode (CallFunction|GetChar) false)
    (Variables|/Script/Engine.PlayerController|SetbShowMouseCursor (Game|GetPlayerController 0) true)
    (Input|SetInputModeGameandUI (Game|GetPlayerController 0) 0 "DoNotLock" false)
    (Default|StartTimer (Variables|/Game/UI/WB_GameplayUI.WB_GameplayUI_C|GetWB_Timer (CallFunction|GetUI)) false)))

(fn ConstructionScript)