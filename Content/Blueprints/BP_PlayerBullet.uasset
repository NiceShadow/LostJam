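; Player bullet actor that flies at a preset velocity with a random pitch spin, using projectile and rotating movement components.
; On box overlap, it destroys itself and any actor whose display name contains "enemy".
; It also destroys only itself on hitting actors tagged "x" or whose names contain an entry from BP_DesignStuff's class-default list.
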(event OnComponentBeginOverlap(Box)
  (params (OverlappedComponent :type Primitive%20Component%20Object%20Reference) (OtherActor :type Actor%20Object%20Reference) (OtherComp :type Primitive%20Component%20Object%20Reference) (OtherBodyIndex :type Integer) (bFromSweep :type Boolean) (SweepResult :type Hit%20Result%20Structure%20%28by%20ref%29))
  (bind _returnvalue (Utilities|GetDisplayName OtherActor))
  (if (Utilities|String|Contains _returnvalue "enemy")
    (Actor|DestroyActor OtherActor)
    (Actor|DestroyActor)
    (else
      (bind _destroyme (CallFunction|IsonList _returnvalue))
      (if (or _destroyme (Actor|ActorHasTag OtherActor "x"))
        (Actor|DestroyActor)))))

(event EventBeginPlay
  (bind _projectilemovement (Variables|Default|GetProjectileMovement))
  (Variables|/Script/Engine.MovementComponent|SetVelocity _projectilemovement (Variables|Default|GetVelocity))
  (Components|Activation|Activate _projectilemovement false)
  (Variables|/Script/Engine.RotatingMovementComponent|SetRotationRate (Variables|Default|GetRotatingMovement) (Math|Rotator|MakeRotator 0.0 (Math|Conversions|ToFloat(Integer) (Math|Random|RandomIntegerinRange 200 400)) 0.0)))

(fn ConstructionScript)

(fn IsonList
  (params (String :type String))
  (for _array_element (Utilities|GetClassDefaults "/Game/Design/BP_DesignStuff.BP_DesignStuff_C")
    (if (Utilities|String|Contains String _array_element)
      (return true)))
  (return false))