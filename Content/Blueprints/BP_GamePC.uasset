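; Player controller for a toast-themed 2D side-scroller that manages the HUD, pause menu, level switching and respawning.
; On BeginPlay it creates the widgets and starts the tutorial.
; StartCertainLevel swaps the active streamed sublevel, teleports the character to the BP_LevelSpawn tagged with its ID, and sets that level's UI and timer.
; Respawn reuses that tagged spawn and restores HP, while pausing is only allowed during play mode.
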(event Custom|StartCertainLevel
  (params (LevelID :type Name))
  (bind _gameplayui_ref (CallFunction|GetUI))
  (bind _gameplayui_ref_2 (CallFunction|GetUI))
  (bind _nontutorialtimeleft (Variables|Default|GetNonTutorialTimeLeft))
  (bind (_days _hours _minutes _seconds) (Math|Timespan|BreakTimespan _nontutorialtimeleft))
  (bind _wb_timer (Variables|/Game/UI/WB_GameplayUI.WB_GameplayUI_C|GetWB_Timer _gameplayui_ref_2))
  (bind _wb_timer_2 (Variables|/Game/UI/WB_GameplayUI.WB_GameplayUI_C|GetWB_Timer _gameplayui_ref))
  (Default|ShowLoadingScreen (CallFunction|GetUI) true)
  (Default|SetPlayMode (CallFunction|GetChar) true)
  (Default|ShowLoadingScreen (CallFunction|GetUI) true)
  (Default|HideHubAnimation (CallFunction|GetUI))
  (if (Utilities|Name|Equal(Name) (Variables|Default|GetActiveLoadedLevel) "None")
    (bind _output_get (Variables|Default|SetActiveLoadedLevel LevelID))
    (Game|LoadStreamLevel(byName) _output_get true)
    (else
      (Game|UnloadStreamLevel(byName) (Variables|Default|GetActiveLoadedLevel) false)
      (bind _output_get_2 (Variables|Default|SetActiveLoadedLevel LevelID))
      (Game|LoadStreamLevel(byName) _output_get_2 true)))
  (CallFunction|TPtoLevel (Variables|Default|GetActiveLoadedLevel))
  (Default|ShowLoadingScreen (CallFunction|GetUI) false)
  (Input|SetInputModeGameOnly (Game|GetPlayerController 0))
  (Variables|Default|SetbShowMouseCursor false)
  (switch name (Variables|Default|GetActiveLoadedLevel)
    (:Default
      (Default|SetTime _wb_timer_2 _minutes _seconds :!label _label)
      (Default|StartTimer _wb_timer_2 true)
      (Default|AddToastUntilFull (CallFunction|GetUI)))
    (:Tutorial
      (Default|SetTime _wb_timer (Variables|Default|GetTutorialMinutes))
      (Default|StartTimer _wb_timer true)
      (Rendering|Components|TextRender|SetText (Variables|/Game/UI/WB_GameplayUI.WB_GameplayUI_C|GetT_LevelName (CallFunction|GetUI)) "Tutorial")
      (Default|AddToastUntilFull (CallFunction|GetUI)))
    (:Level1
      (Rendering|Components|TextRender|SetText (Variables|/Game/UI/WB_GameplayUI.WB_GameplayUI_C|GetT_LevelName (CallFunction|GetUI)) "Level 1")
      (goto _label))
    (:Level2
      (Rendering|Components|TextRender|SetText (Variables|/Game/UI/WB_GameplayUI.WB_GameplayUI_C|GetT_LevelName (CallFunction|GetUI)) "Level 2")
      (goto _label))
    (:Level3
      (Rendering|Components|TextRender|SetText (Variables|/Game/UI/WB_GameplayUI.WB_GameplayUI_C|GetT_LevelName (CallFunction|GetUI)) "Level 3")
      (goto _label))
    (:Breakfast
      (Rendering|Components|TextRender|SetText (Variables|/Game/UI/WB_GameplayUI.WB_GameplayUI_C|GetT_LevelName (CallFunction|GetUI)) "Breakfast"))))

(event EventBeginPlay
  (bind _as2dside_scroller_character (CallFunction|GetChar))
  (bind _gameplayui_ref (CallFunction|GetUI))
  (bind _wb_timer (Variables|/Game/UI/WB_GameplayUI.WB_GameplayUI_C|GetWB_Timer _gameplayui_ref))
  (Class|PlayerController|ActivateTouchInterface)
  (bind _returnvalue (UserInterface|CreateWidget "/Game/UI/WB_GameplayUI.WB_GameplayUI_C"))
  (bind _output_get (Variables|Default|SetGameplayUI_Ref _returnvalue))
  (UserInterface|Viewport|AddtoViewport _output_get 0)
  (Variables|Default|SetbShowMouseCursor false)
  (bind _as2dside_scroller_character_2 (Utilities|Casting|CastTo2DSideScrollerCharacter (Game|GetPlayerCharacter 0)))
  (Default|UpdateToastAmount (Variables|Default|GetGameplayUI_Ref) (Variables|/Game/2DSideScrollerBP/Blueprints/2DSideScrollerCharacter.2DSideScrollerCharacter_C|GetToast _as2dside_scroller_character_2))
  (CallFunction|StartCertainLevel (CallFunction|GetPC) "tutorial")
  (Default|SetTime _wb_timer (Variables|Default|GetTutorialMinutes))
  (Default|StartTimer _wb_timer true)
  (Variables|Default|SetNonTutorialTimeLeft (Utilities|GetClassDefaults "/Game/Design/BP_DesignStuff.BP_DesignStuff_C"))
  (bind _returnvalue_2 (UserInterface|CreateWidget "/Game/UI/WB_PauseMenu.WB_PauseMenu_C"))
  (bind _output_get_2 (Variables|Default|SetPauseMenu_Ref _returnvalue_2))
  (UserInterface|Viewport|AddtoViewport _output_get_2 0)
  (Widget|SetVisibility (Variables|Default|GetPauseMenu_Ref) "Collapsed")
  (Default|UpdateHP _as2dside_scroller_character (Variables|/Game/2DSideScrollerBP/Blueprints/2DSideScrollerCharacter.2DSideScrollerCharacter_C|GetMaxHP _as2dside_scroller_character)))

(event Input|KeyboardEvents|P
  (params (Key :type Key%20Structure :default "None"))
  (:Pressed
    (CallFunction|TogglePaused)))

(event Input|KeyboardEvents|Pause
  (params (Key :type Key%20Structure :default "None"))
  (:Pressed
    (CallFunction|TogglePaused)))

(event Input|KeyboardEvents|Escape
  (params (Key :type Key%20Structure :default "None"))
  (:Pressed
    (CallFunction|TogglePaused)))

(fn ConstructionScript)

(fn TPtoLevel
  (params (LevelID :type Name))
  (bind _outactors (Actor|GetAllActorsOfClasswithTag "/Game/Blueprints/BP_LevelSpawn.BP_LevelSpawn_C" LevelID))
  (Transformation|Teleport (Game|GetPlayerCharacter 0) (Transformation|GetActorLocation (Utilities|Array|Get(acopy) _outactors)) "0, 0, 0"))

(fn SetPaused
  (params (bPaused :type Boolean))
  (if bPaused
    (if (Variables|/Game/2DSideScrollerBP/Blueprints/2DSideScrollerCharacter.2DSideScrollerCharacter_C|GetbPlayMode (CallFunction|GetChar))
      (bind _output_get (Variables|Default|SetbPaused bPaused :!label _label))
      (Game|SetGamePaused _output_get)
      (Widget|SetVisibility (Variables|Default|GetPauseMenu_Ref) (select (Variables|Default|GetbPaused) "Visible" "Collapsed"))
      (Variables|Default|SetbShowMouseCursor (Variables|Default|GetbPaused))
      (if (Variables|Default|GetbPaused)
        (Input|SetInputModeGameandUI self 0 "DoNotLock" false)
        (else
          (Input|SetInputModeGameOnly self))))
    (else
      (goto _label))))

(fn TogglePaused
  (CallFunction|SetPaused (not (Variables|Default|GetbPaused))))

(fn Respawn
  (bind _as2dside_scroller_character (CallFunction|GetChar))
  (Default|PlayDieAnimation (CallFunction|GetUI))
  (bind _outactors (Actor|GetAllActorsOfClasswithTag "/Game/Blueprints/BP_LevelSpawn.BP_LevelSpawn_C" (Variables|Default|GetActiveLoadedLevel)))
  (Transformation|Teleport (Game|GetPlayerCharacter 0) (Transformation|GetActorLocation (Utilities|Array|Get(acopy) _outactors)) "0, 0, 0")
  (Default|UpdateHP _as2dside_scroller_character (Variables|/Game/2DSideScrollerBP/Blueprints/2DSideScrollerCharacter.2DSideScrollerCharacter_C|GetMaxHP _as2dside_scroller_character)))