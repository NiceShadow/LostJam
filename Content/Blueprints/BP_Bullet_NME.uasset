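; BP_Bullet_NME is an enemy bullet that takes its look and size from the DT_BulletsEnemy data table.
; On BeginPlay it reads the Broccoli row when OnlyBroccoli is set, otherwise a random row.
; ApplyData sets the Paper sprite and multiplied Scale, then calls the parent BeginPlay, so parent logic runs only after a row is found and applied.
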(event Custom|ApplyData
  (params (S_BulletsEnemy :type S%20Bullets%20Enemy%20Structure%20%28by%20ref%29))
  (bind (_sprite _size) (Utilities|Struct|BreakS_BulletsEnemy S_BulletsEnemy))
  (Rendering|Components|Sprite|SetSprite (Variables|Default|GetPaperSprite) _sprite)
  (Variables|Default|SetScale (* _size (Variables|Default|GetScaleMultiplier)))
  (|CallParentFunction))

(event EventBeginPlay
  (if (Variables|Default|GetbOnlyBroccoli)
    (bind _returnvalue (Utilities|GetDataTableRow "/Game/Blueprints/DT_BulletsEnemy.DT_BulletsEnemy" "Broccoli")
      (:then
        (CallFunction|ApplyData _returnvalue)))
    (else
      (bind _outrownames (DataTable|GetDataTableRowNames "/Game/Blueprints/DT_BulletsEnemy.DT_BulletsEnemy"))
      (bind _returnvalue_2 (Utilities|GetDataTableRow "/Game/Blueprints/DT_BulletsEnemy.DT_BulletsEnemy" (Utilities|Array|Get(acopy) _outrownames (Math|Random|RandomIntegerinRange 0 (Utilities|Array|LastIndex _outrownames))))
        (:then
          (CallFunction|ApplyData _returnvalue_2))))))

(fn ConstructionScript
  (|CallParentFunction))