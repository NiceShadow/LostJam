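; BP_Enemy is an enemy actor that repeatedly fires bullets horizontally toward the player.
; On BeginPlay it starts a looping timer, with its interval read from the BP_DesignStuff class defaults, that calls SpawnBullet.
; SpawnBullet spawns a BP_EnemyBullet at the BulletSpawn component, choosing a fixed-speed velocity along positive or negative X by comparing its position with the player character's.
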(event EventBeginPlay
  (Utilities|Time|SetTimerbyFunctionName 0 "SpawnBullet" (Utilities|GetClassDefaults "/Game/Design/BP_DesignStuff.BP_DesignStuff_C") true -0.8))

(fn ConstructionScript)

(fn SpawnBullet
  (Game|SpawnActorfromClass "/Game/Blueprints/BP_EnemyBullet.BP_EnemyBullet_C" (Transformation|GetWorldTransform (Variables|Default|GetBulletSpawn)) "Undefined" self (select (> (.X (Math|Vector|BreakVector (Transformation|GetActorLocation))) (.X (Math|Vector|BreakVector (Transformation|GetActorLocation (Game|GetPlayerCharacter 0))))) "-300.000000, 0, 0" "300.000000, 0, 0") 0))