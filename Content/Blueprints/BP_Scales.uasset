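; A weighing scale prop that sinks and swings its needle while the player character stands on it.
; Box overlap begin and end call ScaleDown, which plays or reverses two timelines.
; One timeline lerps the paper sprite downward, and the other lerps the Arrow's roll.
; The arrow's alpha is clamped to 0–1 only in reverse, so any overshoot in the curve shows only on the way down.
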(event OnComponentBeginOverlap(Box)
  (params (OverlappedComponent :type Primitive%20Component%20Object%20Reference) (OtherActor :type Actor%20Object%20Reference) (OtherComp :type Primitive%20Component%20Object%20Reference) (OtherBodyIndex :type Integer) (bFromSweep :type Boolean) (SweepResult :type Hit%20Result%20Structure%20%28by%20ref%29))
  (if (== OtherActor (Game|GetPlayerCharacter 0))
    (CallFunction|ScaleDown true)))

(event OnComponentEndOverlap(Box)
  (params (OverlappedComponent :type Primitive%20Component%20Object%20Reference) (OtherActor :type Actor%20Object%20Reference) (OtherComp :type Primitive%20Component%20Object%20Reference) (OtherBodyIndex :type Integer))
  (if (== OtherActor (Game|GetPlayerCharacter 0))
    (CallFunction|ScaleDown false)))

(event Custom|ScaleDown
  (params (bDown :type Boolean))
  (if bDown
    (Utilities|FlowControl|Sequence
      (:then_0
        (bind _alpha (Timeline|Timeline_0 Play)
          (:Update
            (Transformation|SetRelativeLocation (Variables|Default|GetPaperSprite1) (Math|Vector|MakeVector 0.0 3.0 (Math|Float|Lerp 0.0 -25.0 _alpha)) false false))))
      (:then_1
        (bind (_direction _alpha_2) (Timeline|Timeline_1 Play)
          (:Update
            (Transformation|SetRelativeRotation (Variables|Default|GetArrow) (Math|Rotator|MakeRotator (Math|Float|Lerp 2e+01 -6e+01 (select (Utilities|Enum|Equal(Enum) _direction "Backward") (Math|Float|Clamp(Float) _alpha_2) _alpha_2)) 0.0 9e+01) false false)))))
    (else
      (Utilities|FlowControl|Sequence
        (:then_0
          (Timeline|Timeline_0 Reverse))
        (:then_1
          (Timeline|Timeline_1 Reverse))))))

(fn ConstructionScript)