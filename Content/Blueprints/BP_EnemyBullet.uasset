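; BP_EnemyBullet is a 2D Paper sprite enemy projectile with a randomized look, size and spin.
; On BeginPlay it passes its Velocity variable to ProjectileMovement and gives the sprite a random pitch spin through RotatingMovement.
; It picks a random DT_BulletsEnemy row for the sprite and base size, applies random scale variation, then matches the Box's scale to the sprite.
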(event EventBeginPlay
  (bind _projectilemovement (Variables|Default|GetProjectileMovement))
  (Variables|/Script/Engine.MovementComponent|SetVelocity _projectilemovement (Variables|Default|GetVelocity))
  (Components|Activation|Activate _projectilemovement false)
  (Components|Movement|SetUpdatedComponent (Variables|Default|GetRotatingMovement) (Variables|Default|GetPaperSprite))
  (Variables|/Script/Engine.RotatingMovementComponent|SetRotationRate (Variables|Default|GetRotatingMovement) (Math|Rotator|MakeRotator 0.0 (* (Math|Random|RandomIntegerinRange 200 400) 1.0) 0.0))
  (bind _outrownames (DataTable|GetDataTableRowNames "/Game/Blueprints/DT_BulletsEnemy.DT_BulletsEnemy"))
  (bind _returnvalue (Utilities|GetDataTableRow "/Game/Blueprints/DT_BulletsEnemy.DT_BulletsEnemy" (Utilities|Array|Get(acopy) _outrownames (Math|Random|RandomIntegerinRange 0 (- (Utilities|Array|Length _outrownames) 1))))
    (:then
      (Rendering|Components|Sprite|SetSprite (Variables|Default|GetPaperSprite) (.Sprite (Utilities|Struct|BreakS_BulletsEnemy _returnvalue)))
      (Transformation|SetRelativeScale3D (Variables|Default|GetPaperSprite) (Math|Conversions|ToVector(Float) (* (.Size (Utilities|Struct|BreakS_BulletsEnemy _returnvalue)) (Math|Random|RandomFloatinRange 1.2 0.7))))
      (Transformation|SetRelativeScale3D (Variables|Default|GetBox) (Variables|/Script/Engine.SceneComponent|GetRelativeScale3D (Variables|Default|GetPaperSprite))))))

(fn ConstructionScript)