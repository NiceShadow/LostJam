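; A pancake jam mine that detonates when an actor overlaps it, with no filter on the overlapping actor in the graph.
; Each child component of Scene acts as a muzzle, spawning a jam bullet launched along its forward vector and set to ignore BP_Enemy.
; A cheering sound, particle flash and camera shake accompany the burst.
; A timeline then shrinks the sprite to zero and destroys the actor.
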(event Collision|EventActorBeginOverlap
  (params (OtherActor :type Actor%20Object%20Reference))
  (for _array_element (Components|GetChildrenComponents (Variables|Default|GetScene) false)
    (Game|SpawnActorfromClass "/Game/Blueprints/BP_Bullet_PancakeJam.BP_Bullet_PancakeJam_C" (Transformation|GetWorldTransform _array_element) "Undefined" 0 (Utilities|Array|MakeArray "/Game/Blueprints/BP_Enemy.BP_Enemy_C") (* (Math|Vector|GetForwardVector (.Rotation (Math|Transform|BreakTransform (Transformation|GetWorldTransform _array_element)))) 700) 0))
  (Audio|SpawnSoundatLocation "/Game/LostSounds/cheering1_Cue.cheering1_Cue" (Transformation|GetActorLocation) "0, 0, 0" 1.0 1.0 0.0 "/Game/LostSounds/NME_Atten.NME_Atten" 0)
  (Effects|SpawnEmitteratLocation "/Game/AdvancedMagicFX13/Particles/P_ky_flash2.P_ky_flash2" (+ (Transformation|GetActorLocation) "0, 0,50.000000") "0, 0, 0" "2.000000,2.000000,2.000000")
  (Class|PlayerCameraManager|PlayCameraShake (Game|GetPlayerCameraManager 0) "/Game/Blueprints/BP_CamShake2.BP_CamShake2_C" 1.5 "CameraLocal" "0, 0, 0")
  (Variables|Default|SetScaleBeforeDestruction (.X (Math|Vector|BreakVector (Variables|/Script/Engine.SceneComponent|GetRelativeScale3D (Variables|Default|GetPaperSprite)))))
  (bind _alpha (Timeline|Timeline_0 PlayFromStart)
    (:Update
      (Transformation|SetRelativeScale3D (Variables|Default|GetPaperSprite) (Math|Conversions|ToVector(Float) (Math|Float|Lerp (Variables|Default|GetScaleBeforeDestruction) 0.0 _alpha))))
    (:Finished
      (Actor|DestroyActor))))

(fn ConstructionScript)