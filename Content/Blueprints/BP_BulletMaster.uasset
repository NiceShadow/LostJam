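; BP_BulletMaster is a 2D sprite projectile that moves at a set velocity with randomized spin and scale.
; On overlap, a name match against BP_DesignStuff's BulletDestroyList or an "x" tag destroys it without notifying the other actor.
; Otherwise, unless the actor's class is ignored or its own, it sends OnBulletHitMessage with its BulletID and destroys itself.
; Destruction disables collision, plays a hit sound and shrinks the sprite via timeline before removing the actor.
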(event OnComponentBeginOverlap(Box)
  (params (OverlappedComponent :type Primitive%20Component%20Object%20Reference) (OtherActor :type Actor%20Object%20Reference) (OtherComp :type Primitive%20Component%20Object%20Reference) (OtherBodyIndex :type Integer) (bFromSweep :type Boolean) (SweepResult :type Hit%20Result%20Structure%20%28by%20ref%29))
  (CallFunction|OnOverlap OtherActor))

(event Custom|DestroyAnimated
  (Collision|SetActorEnableCollision false)
  (Audio|SpawnSoundatLocation "/Game/LostSounds/hit2.hit2" (Transformation|GetActorLocation) "0, 0, 0" 0.1 0.6 0.0 "/Game/LostSounds/NME_Atten.NME_Atten" 0)
  (Variables|Default|SetScaleBeforeDestruction (.X (Math|Vector|BreakVector (Variables|/Script/Engine.SceneComponent|GetRelativeScale3D (Variables|Default|GetPaperSprite)))))
  (bind _alpha (Timeline|Timeline_Destroy PlayFromStart)
    (:Update
      (Transformation|SetRelativeScale3D (Variables|Default|GetPaperSprite) (Math|Conversions|ToVector(Float) (Math|Float|Lerp (Variables|Default|GetScaleBeforeDestruction) 0.0 _alpha))))
    (:Finished
      (Actor|DestroyActor))))

(event EventBeginPlay
  (Variables|/Script/Engine.MovementComponent|SetVelocity (Variables|Default|GetProjectileMovement) (Variables|Default|GetVelocity))
  (Components|Activation|Activate (Variables|Default|GetProjectileMovement) false)
  (Variables|/Script/Engine.RotatingMovementComponent|SetRotationRate (Variables|Default|GetRotatingMovement) (Math|Rotator|MakeRotator 0.0 (Math|Conversions|ToFloat(Integer) (Math|Random|RandomIntegerinRange (Math|Integer|Min(Integer) (Math|Float|Truncate (+ (.Pitch (Math|Rotator|BreakRotator (Variables|/Script/Engine.RotatingMovementComponent|GetRotationRate (Variables|Default|GetRotatingMovement)))) -1.2e+02)) (Math|Float|Truncate (+ (.Pitch (Math|Rotator|BreakRotator (Variables|/Script/Engine.RotatingMovementComponent|GetRotationRate (Variables|Default|GetRotatingMovement)))) 1.2e+02))) (Math|Integer|Max(Integer) (Math|Float|Truncate (+ (.Pitch (Math|Rotator|BreakRotator (Variables|/Script/Engine.RotatingMovementComponent|GetRotationRate (Variables|Default|GetRotatingMovement)))) -1.2e+02)) (Math|Float|Truncate (+ (.Pitch (Math|Rotator|BreakRotator (Variables|/Script/Engine.RotatingMovementComponent|GetRotationRate (Variables|Default|GetRotatingMovement)))) 1.2e+02))))) 0.0))
  (Transformation|SetRelativeScale3D (Variables|Default|GetPaperSprite) (Math|Conversions|ToVector(Float) (* (Variables|Default|GetScale) (Math|Random|RandomFloatinRange (- 1.0 (Variables|Default|GetScaleVariation)) (+ 1.0 (Variables|Default|GetScaleVariation))))))
  (Transformation|SetRelativeScale3D (Variables|Default|GetBox) (Variables|/Script/Engine.SceneComponent|GetRelativeScale3D (Variables|Default|GetPaperSprite))))

(fn ConstructionScript)

(fn IsonList
  (params (String :type String))
  (for _array_element (.BulletDestroyList (Utilities|GetClassDefaults "/Game/Design/BP_DesignStuff.BP_DesignStuff_C"))
    (if (Utilities|String|Contains String _array_element)
      (return true)))
  (return false))

(fn OnOverlap
  (params (ActorOverlap :type Actor%20Object%20Reference))
  (bind _destroyme (CallFunction|IsonList (Utilities|GetDisplayName ActorOverlap)))
  (if (or _destroyme (Actor|ActorHasTag ActorOverlap "x"))
    (CallFunction|DestroyAnimated)
    (elif (and (not (Utilities|Array|ContainsItem (Variables|Default|GetClassesToIgnore) (Utilities|GetClass ActorOverlap))) (not (== (Utilities|GetClass ActorOverlap) (Utilities|GetClass self))))
      (Class|BPIBullet|OnBulletHit(Message) ActorOverlap (Variables|Default|GetBulletID))
      (CallFunction|DestroyAnimated))))